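; BP_WinArea is a Blueprint that handles the player's win sequence.
; On BeginPlay it binds an event to the OnWin dispatcher.
; The GameWon event ignores the first player's move input and waits briefly, then shows WBP_WinScreen with UI-only input and a visible mouse cursor.
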(event Custom|GameWon
  (Input|SetIgnoreMoveInput (Game|GetPlayerController 0) true)
  (Utilities|FlowControl|Delay 2.0)
  (bind _returnvalue (UserInterface|CreateWidget "/Game/Blueprints/WBP_WinScreen.WBP_WinScreen_C" (Game|GetPlayerController 0)))
  (UserInterface|Viewport|AddtoViewport _returnvalue 0)
  (Input|SetInputModeUIOnly (Game|GetPlayerController 0) 0 "DoNotLock" false)
  (Variables|/Script/Engine.PlayerController|SetbShowMouseCursor (Game|GetPlayerController 0) true))

(event EventBeginPlay
  (EventDispatchers|BindEventtoOnWin (EventDispatchers|CreateEvent :!event Custom|GameWon)))

(fn ConstructionScript)